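; Base character Blueprint using the Gameplay Ability System, with health UI, punch hit detection and a K-key ragdoll kill.
; BeginPlay applies GE_Damage to itself, then creates a viewport health widget for player 0's pawn or binds the enemy health widget component for others.
; HandlePunch sphere-overlaps other characters at the right hand and sends the first hit to its instigator as a Weapon.Hit gameplay event with target data.
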(event Custom|HandlePunch
  (bind _returnvalue (Game|GetInstigator))
  (bind _outactors (Collision|SphereOverlapActors (Transformation|GetSocketLocation (Variables|Character|GetMesh) "RightHand") 5e+01 (Utilities|Array|MakeArray "ObjectTypeQuery3") "BP_CppBaseCharacter_C" (Utilities|Array|MakeArray self)))
  (if (Utilities|Array|IsValidIndex _outactors)
    (Ability|SendGameplayEventtoActor _returnvalue "(TagName=\"Weapon.Hit\")" (Utilities|Struct|MakeGameplayEventData "(TagName=\"\")" _returnvalue (Utilities|Array|Get(acopy) _outactors) 0 0 "()" "(GameplayTags=)" "(GameplayTags=)" 0.0 (Ability|TargetData|AbilityTargetDatafromActor (Utilities|Array|Get(acopy) _outactors))))))

(event EventBeginPlay
  (bind _healthwidgetifennemy (Variables|Default|GetHealthWidgetIfEnnemy))
  (GameplayEffects|ApplyGameplayEffectToSelf :self (Variables|Default|GetAbilitySystemComponent) :GameplayEffectClass "/Game/Blueprints/Abilities/GE_Damage.GE_Damage_C" :Level 1.0)
  (if (== (Game|Player|GetPlayerPawn 0) (Class|PawnMovementComponent|GetPawnOwner (Variables|Character|GetCharacterMovement self)))
    (Components|Activation|Deactivate _healthwidgetifennemy)
    (Rendering|SetVisibility _healthwidgetifennemy false false)
    (bind _returnvalue (UserInterface|CreateWidget "/Game/UI/WBP_Health.WBP_Health_C" (Game|GetPlayerController 0)))
    (bind _output_get (Variables|Default|SetHealthUI _returnvalue))
    (UserInterface|Viewport|AddtoViewport _output_get 0)
    (else
      (bind _aswbp_ennemy_health (Utilities|Casting|CastToWBP_EnnemyHealth (UserInterface|GetWidget (Variables|Default|GetHealthWidgetIfEnnemy))))
      (Default|SetOwner _aswbp_ennemy_health self))))

(event Input|KeyboardEvents|K
  (params (Key :type Key%20Structure :default "None"))
  ;[1 1 1] Kill
  (:Pressed
    (Pawn|Components|CharacterMovement|DisableMovement (Variables|Character|GetCharacterMovement))
    (Collision|SetCollisionProfileName (Variables|Character|GetMesh) "Ragdoll" true :!class /Script/Engine.PrimitiveComponent)
    (Class|SkeletalMeshComponent|SetAllBodiesSimulatePhysics (Variables|Character|GetMesh) true)))

(fn ConstructionScript)