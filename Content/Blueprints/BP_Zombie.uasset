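; Zombie enemy that runs the BT_Zombie behavior tree and restarts the level when it catches the player.
; AI perception writes the target to the blackboard, delaying target loss briefly, while chase events play and fade music.
; CatchPlayer eases player and camera toward the zombie, plays a montage, fades out, then reloads.
; Rocky input handlers and disconnected older sense, chase and wander logic remain in the graph.
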(event OnTargetPerceptionUpdated(AIPerception)
  (params (Actor :type Actor%20Object%20Reference) (Stimulus :type AI%20Stimulus%20Structure))
  (bind _bsuccessfullysensed (Utilities|Struct|BreakAIStimulus Stimulus))
  (bind _returnvalue (AI|GetBlackboard 0))
  (AI|Components|Blackboard|SetValueasObject _returnvalue (Utilities|Name|MakeLiteralName "TargetActor") Actor)
  (Development|PrintString (Utilities|String|ToString(Boolean) _bsuccessfullysensed))
  (if _bsuccessfullysensed
    _
    (else
      (Utilities|FlowControl|RetriggerableDelay 2.0)))
  (AI|Components|Blackboard|SetValueasBool _returnvalue (Utilities|Name|MakeLiteralName "TargetAcquired") _bsuccessfullysensed))

(event OnSeePawn(PawnSensing)
  (params (Pawn :type Pawn%20Object%20Reference)))

(event Custom|CatchPlayer
  (bind _returnvalue (Game|GetPlayerController 0))
  (bind _asbp_rocky_character (Utilities|Casting|CastToBP_RockyCharacter (Game|GetPlayerCharacter 0)))
  (Transformation|SetActorRotation _asbp_rocky_character (Math|Interpolation|RInterpTo (Transformation|GetActorRotation _asbp_rocky_character) (Math|Rotator|FindLookatRotation (Transformation|GetActorLocation _asbp_rocky_character) (Transformation|GetActorLocation)) (Utilities|Time|GetWorldDeltaSeconds) 5.0))
  (Pawn|SetControlRotation _returnvalue (Math|Interpolation|RInterpTo (Pawn|GetControlRotation _returnvalue :!class /Script/Engine.Controller) (Math|Rotator|FindLookatRotation (Transformation|GetActorLocation _asbp_rocky_character) (Transformation|GetActorLocation)) (Utilities|Time|GetWorldDeltaSeconds) 0.0))
  (Animation|Montage|PlayMontage 0 0
    (:then
      (Utilities|FlowControl|Delay 1.0)
      (CameraFades|StartCameraFade :self (Game|GetPlayerCameraManager 0) :ToAlpha 1.0 :Duration 2.0 :bShouldFadeAudio true :bHoldWhenFinished true)
      (Utilities|FlowControl|Delay 2.1)
      (bind _returnvalue_2 (Game|GetCurrentLevelName true))
      (Game|OpenLevel(byName) (Utilities|String|StringToName _returnvalue_2)))))

(event Custom|ChasePlayer
  (Audio|Components|Audio|Play (Variables|Default|GetMusic) 0.0))

(event Custom|StopChasingPlayer
  (Audio|Components|Audio|FadeOut (Variables|Default|GetMusic) 2.0 0.0 "Linear" :!class /Script/Engine.AudioComponent))

(event Input|EnhancedActionEvents|EnhancedInputActionIA_RockyJump
  (params (ActionValue :type Boolean) (ElapsedSeconds :type Float%20%28double-precision%29) (TriggeredSeconds :type Float%20%28double-precision%29) (InputAction :type Input%20Action%20Object%20Reference :default "/Game/Input/IA_RockyJump.IA_RockyJump"))
  (:Triggered
    (Character|Jump))
  (:Completed
    (Character|StopJumping)))

(event Input|EnhancedActionEvents|EnhancedInputActionIA_RockyMove
  (params (ActionValue :type Vector%202D%20Structure) (ElapsedSeconds :type Float%20%28double-precision%29) (TriggeredSeconds :type Float%20%28double-precision%29) (InputAction :type Input%20Action%20Object%20Reference :default "/Game/Input/IA_RockyMove.IA_RockyMove"))
  (bind _returnvalue (Pawn|GetControlRotation :!class /Script/Engine.Pawn))
  (:Triggered
    (Pawn|Input|AddMovementInput (Math|Vector|GetRightVector (Math|Rotator|MakeRotator (.roll _returnvalue) 0.0 (.yaw _returnvalue))) (.x ActionValue) false)
    (Pawn|Input|AddMovementInput (Math|Vector|GetForwardVector (Math|Rotator|MakeRotator 0.0 0.0 (.yaw (Pawn|GetControlRotation :!class /Script/Engine.Pawn)))) (.y ActionValue) false)))

(event Input|EnhancedActionEvents|EnhancedInputActionIA_RockyCameraLook
  (params (ActionValue :type Vector%202D%20Structure) (ElapsedSeconds :type Float%20%28double-precision%29) (TriggeredSeconds :type Float%20%28double-precision%29) (InputAction :type Input%20Action%20Object%20Reference :default "/Game/Input/IA_RockyCameraLook.IA_RockyCameraLook"))
  (:Triggered
    (Pawn|Input|AddControllerYawInput (.x ActionValue))
    (Pawn|Input|AddControllerPitchInput (.y ActionValue))))

(event EventBeginPlay
  (bind _returnvalue (AddComponent|AddAudioComponent false))
  (Audio|Components|Audio|Stop _returnvalue)
  (Variables|Default|SetMusic _returnvalue)
  (AI|RunBehaviorTree (AI|GetAIController self) "/Game/Blueprints/BT_Zombie.BT_Zombie")
  (Development|PrintText "Hello" true true "(R=0.000000,G=0.660000,B=1.000000,A=1.000000)" 1e+01))

(event EventTick
  (params (DeltaSeconds :type Float%20%28single-precision%29)))

(fn ConstructionScript)