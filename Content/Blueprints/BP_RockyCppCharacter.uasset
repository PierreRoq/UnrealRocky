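; BP_RockyCppCharacter is a character Blueprint that uses the Gameplay Ability System for punch hit detection.
; On BeginPlay it applies GE_Damage to itself.
; HandlePunch runs a sphere overlap at the right-hand socket for other characters of the same class.
; The first hit is sent to the character's instigator as a Weapon.Hit gameplay event carrying target data, leaving any response to listeners outside this graph.
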(event Custom|HandlePunch
  (bind _returnvalue (Game|GetInstigator))
  (bind _outactors (Collision|SphereOverlapActors (Transformation|GetSocketLocation (Variables|Character|GetMesh) "RightHand") 5e+01 (Utilities|Array|MakeArray "ObjectTypeQuery3") "BP_RockyCppCharacter_C" (Utilities|Array|MakeArray self)))
  (if (Utilities|Array|IsValidIndex _outactors)
    (Ability|SendGameplayEventtoActor _returnvalue "(TagName=\"Weapon.Hit\")" (Utilities|Struct|MakeGameplayEventData "(TagName=\"\")" _returnvalue (Utilities|Array|Get(acopy) _outactors) 0 0 "()" "(GameplayTags=)" "(GameplayTags=)" 0.0 (Ability|TargetData|AbilityTargetDatafromActor (Utilities|Array|Get(acopy) _outactors))))))

(event EventBeginPlay
  (GameplayEffects|ApplyGameplayEffectToSelf :self (Variables|Default|GetAbilitySystemComponent) :GameplayEffectClass "/Game/Blueprints/Abilities/GE_Damage.GE_Damage_C" :Level 1.0))

(fn ConstructionScript)