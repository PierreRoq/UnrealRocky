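; Table actor that spits out an art mesh whenever a BP_CppBaseCharacter hits it.
; Each hit spawns a StaticMeshActor just above the table, assigns ArtMesh, enables physics and applies an upward unit-vector force.
; A DoOnce gates the SWFoom0 whoosh sound, resetting when the audio finishes so plays do not overlap, while spawning itself is not throttled.
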(event OnComponentHit(Table)
  (params (HitComponent :type Primitive%20Component%20Object%20Reference) (OtherActor :type Actor%20Object%20Reference) (OtherComp :type Primitive%20Component%20Object%20Reference) (NormalImpulse :type Vector :default "0, 0, 0") (Hit :type Hit%20Result%20Structure%20%28by%20ref%29))
  (bind _instigator (Variables|Actor|GetInstigator))
  (Utilities|Casting|CastToBP_CppBaseCharacter OtherActor)
  (bind _returnvalue (Game|SpawnActorfromClass "/Script/Engine.StaticMeshActor" (Math|Transform|MakeTransform (+ (Transformation|GetActorLocation) "0.000000,0.000000,50.000000") "0, 0, 0" "1.000000,1.000000,1.000000") "Undefined" _instigator _instigator))
  (Transformation|SetMobility (Variables|/Script/Engine.StaticMeshActor|GetStaticMeshComponent _returnvalue) "Movable")
  (Physics|SetSimulatePhysics (Variables|/Script/Engine.StaticMeshActor|GetStaticMeshComponent _returnvalue) true)
  (Components|StaticMesh|SetStaticMesh (Variables|/Script/Engine.StaticMeshActor|GetStaticMeshComponent _returnvalue) (Variables|Default|GetArtMesh))
  (Physics|AddForce (Variables|/Script/Engine.StaticMeshActor|GetStaticMeshComponent _returnvalue) (Math|Vector|GetUpVector "0, 0, 0") "None" false)
  (Utilities|FlowControl|DoOnce false
    (:Completed
      (Audio|Components|Audio|Play (Variables|Default|GetSW_foom_0) 0.0))))

(event Custom|OnWooshSoundCompleted
  (Utilities|FlowControl|DoOnce false) ; enters at Reset
)

(event EventBeginPlay
  (EventDispatchers|BindEventtoOnAudioFinished (Variables|Default|GetSW_foom_0) (delegate Custom|OnWooshSoundCompleted)))

(fn ConstructionScript)